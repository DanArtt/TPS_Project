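; Third-person shooter player character with camera-relative movement, interpolated sprint speed, crouch toggle and zoomed rifle aiming.
; A per-tick trace highlights items, the pickup input messages them through an interface, and WeaponPickUp spawns an AK47 or M4A1 onto its holster socket.
; A slow-motion radial HUD toggles equip state and plays montages, while separate equip events swap hand/back sockets.
; Fire and reload inputs forward to the weapons.
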(event Custom|WeaponPickUp
  (params (CurrentWeapon :type Actor%20Object%20Reference))
  ;[1 1 1] PickUp
  ;;[0 1 0] WeaponPickUp
  (bind _output_get (Variables|Default|SetCurrentWeapon CurrentWeapon))
  (bind _asweapon_base (Utilities|Casting|CastToWeaponBase _output_get))
  (bind _output_get_2 (Variables|Default|SetWeaponBaseRef _asweapon_base))
  (switch Utilities|FlowControl|Switch|SwitchonWeaponType (.WeaponType (Utilities|Struct|BreakWeaponInfo (Variables|/Game/Itens/ItensBP/WeaponItem/WeaponBase.WeaponBase_C|GetWeaponInfo _output_get_2)))
    (:NewEnumerator1
      (bind _returnvalue (Game|SpawnActorfromClass (.ItemClass (Utilities|Struct|BreakWeaponInfo (Variables|/Game/Itens/ItensBP/WeaponItem/WeaponBase.WeaponBase_C|GetWeaponInfo _output_get_2))) (Transformation|GetSocketTransform (Variables|Character|GetMesh) (.UnEquipWeapon (Utilities|Struct|BreakWeaponInfo (Variables|/Game/Itens/ItensBP/WeaponItem/WeaponBase.WeaponBase_C|GetWeaponInfo _output_get_2))) "RTS_World") "Undefined" 0 0))
      (bind _output_get_3 (Variables|Default|SetAK47 _returnvalue))
      (Transformation|AttachComponentToComponent _output_get_3 (Variables|Character|GetMesh) (.UnEquipWeapon (Utilities|Struct|BreakWeaponInfo (Variables|/Game/Itens/ItensBP/WeaponItem/WeaponBase.WeaponBase_C|GetWeaponInfo _output_get_2))) "SnapToTarget" "SnapToTarget" "SnapToTarget" true)
      (Actor|DestroyActor _output_get_2))
    (:NewEnumerator2
      (bind _returnvalue_2 (Game|SpawnActorfromClass (.ItemClass (Utilities|Struct|BreakWeaponInfo (Variables|/Game/Itens/ItensBP/WeaponItem/WeaponBase.WeaponBase_C|GetWeaponInfo _output_get_2))) (Transformation|GetSocketTransform (Variables|Character|GetMesh) (.UnEquipWeapon (Utilities|Struct|BreakWeaponInfo (Variables|/Game/Itens/ItensBP/WeaponItem/WeaponBase.WeaponBase_C|GetWeaponInfo _output_get_2))) "RTS_World") "Undefined" 0 0))
      (bind _output_get_4 (Variables|Default|SetM4A1 _returnvalue_2))
      (Transformation|AttachComponentToComponent _output_get_4 (Variables|Character|GetMesh) (.UnEquipWeapon (Utilities|Struct|BreakWeaponInfo (Variables|/Game/Itens/ItensBP/WeaponItem/WeaponBase.WeaponBase_C|GetWeaponInfo _output_get_2))) "SnapToTarget" "SnapToTarget" "SnapToTarget" true)
      (Actor|DestroyActor _output_get_2))))

(event Custom|EquipAK47
  ;[1 1 1] Armas
  ;;[1 0 0] Equipar AK47
  (if (Utilities|IsValid (Variables|Default|GetAK47))
    (if (and (Variables|Default|GetEquipWeapon) (Variables|Default|GetEquipAK47?))
      (Transformation|AttachComponentToComponent (Variables|Default|GetAK47) (Variables|Character|GetMesh) "AK47" "SnapToTarget" "SnapToTarget" "SnapToTarget" true)
      (if (Utilities|IsValid (Variables|Default|GetM4A1))
        (if (Variables|Default|GetEquipM4A1?)
          (Transformation|AttachComponentToComponent (Variables|Default|GetM4A1) (Variables|Character|GetMesh) "BackM4" "SnapToTarget" "SnapToTarget" "SnapToTarget" true)
          (Variables|Default|SetEquipM4A1? false)))
      (else
        (Transformation|AttachComponentToComponent (Variables|Default|GetAK47) (Variables|Character|GetMesh) "BackAK47" "SnapToTarget" "SnapToTarget" "SnapToTarget" true)))))

(event Custom|EquipM4A1
  ;[1 1 1] Armas
  ;;[1 0 0] Equipar M4
  (if (Utilities|IsValid (Variables|Default|GetM4A1))
    (if true
      (if (and (Variables|Default|GetEquipWeapon) (Variables|Default|GetEquipM4A1?))
        (Transformation|AttachComponentToComponent (Variables|Default|GetM4A1) (Variables|Character|GetMesh) "M4A1" "SnapToTarget" "SnapToTarget" "SnapToTarget" true)
        (if (Utilities|IsValid (Variables|Default|GetAK47))
          (if (Variables|Default|GetEquipAK47?)
            (Transformation|AttachComponentToComponent (Variables|Default|GetAK47) (Variables|Character|GetMesh) "BackAK47" "SnapToTarget" "SnapToTarget" "SnapToTarget" true)
            (Variables|Default|SetEquipAK47? false)))
        (else
          (Transformation|AttachComponentToComponent (Variables|Default|GetM4A1) (Variables|Character|GetMesh) "BackM4" "SnapToTarget" "SnapToTarget" "SnapToTarget" true))))))

(event EventTick
  (params (DeltaSeconds :type Float%20%28single-precision%29))
  ;[1 1 1] Event Tick
  (CallFunction|ItemDecoration))

(event EventBeginPlay
  ;[1 1 1] Begin Play
  (Utilities|FlowControl|Sequence
    (:then_0
      (Utilities|MainHUDTPS))))

(event Input|ActionEvents|InputActionRunning
  (params (Key :type Key%20Structure :default "None"))
  ;[1 1 1] Movement Character
  ;;[0 0 0] Control Running
  (:Pressed
    (Utilities|Running :!label _label))
  (:Released
    (goto _label StopRun)))

(event Input|ActionEvents|InputActionWeaponAin
  (params (Key :type Key%20Structure :default "None"))
  (bind _springarm (Variables|Default|GetSpringArm))
  ;[1 1 1] Armas
  ;;[1 0 0] Mirar
  (:Pressed
    (if (Variables|Default|GetEquipWeapon)
      (Variables|Default|SetAinRifle? true)
      (Variables|Default|SetbUseControllerRotationYaw true)
      (bind _zoomweapon (Timeline|ZoomWeapon PlayFromStart)
        (:Update
          (Variables|/Script/Engine.CameraComponent|SetFieldOfView (Variables|Default|GetCamera) _zoomweapon)
          (Variables|/Script/Engine.CharacterMovementComponent|SetbOrientRotationToMovement (Variables|Character|GetCharacterMovement) false)
          (Variables|/Script/Engine.SpringArmComponent|SetbEnableCameraLag _springarm false)
          (Variables|/Script/Engine.SpringArmComponent|SetCameraRotationLagSpeed _springarm 3e+01)))))
  (:Released
    (Variables|Default|SetAinRifle? false)
    (Variables|Default|SetbUseControllerRotationYaw false)
    (bind _zoomweapon_2 (Timeline|ZoomWeaponOut ReverseFromEnd)
      (:Update
        (Variables|/Script/Engine.CameraComponent|SetFieldOfView (Variables|Default|GetCamera) _zoomweapon_2)
        (Variables|/Script/Engine.CharacterMovementComponent|SetbOrientRotationToMovement (Variables|Character|GetCharacterMovement) true)
        (Variables|/Script/Engine.SpringArmComponent|SetbEnableCameraLag _springarm false)
        (Variables|/Script/Engine.SpringArmComponent|SetCameraRotationLagSpeed _springarm 0.0)
        (if (not (Variables|Default|GetAinRifle?))
          (if (Utilities|IsValid (Variables|Default|GetAK47))
            (Default|FireReleased (Variables|Default|GetAK47)))
          (if (not (Variables|Default|GetAinRifle?))
            (if (Utilities|IsValid (Variables|Default|GetM4A1))
              (Default|FireReleased (Variables|Default|GetM4A1)))))))))

(event Input|ActionEvents|InputActionSelectWeapon
  (params (Key :type Key%20Structure :default "None"))
  (bind _returnvalue (Game|GetPlayerController 0))
  (bind _returnvalue_2 (Game|GetPlayerController 0))
  ;[1 1 1] HUD
  ;;[0 0 1] HUD Select
  (:Pressed
    (Variables|Default|SetWindowsIsOpen? true)
    (Utilities|Time|SetGlobalTimeDilation 0.1)
    (bind _returnvalue_3 (UserInterface|CreateWidget "/Game/Itens/HUD/HUDCircular.HUDCircular_C"))
    (Default|StartSelect _returnvalue_3)
    (bind _output_get (Variables|Default|SetHUDCircularRef _returnvalue_3))
    (UserInterface|Viewport|AddtoViewport _output_get 0)
    (Variables|/Script/Engine.PlayerController|SetbShowMouseCursor _returnvalue true)
    (Input|SetIgnoreLookInput _returnvalue true)
    (Input|SetInputModeGameandUI _returnvalue _output_get "DoNotLock" false))
  (:Released
    (Variables|Default|SetWindowsIsOpen? false)
    (Utilities|Time|SetGlobalTimeDilation 1.0)
    (Default|EndSelect (Variables|Default|GetHUDCircularRef))
    (Widget|RemovefromParent (Variables|Default|GetHUDCircularRef))
    (Variables|/Script/Engine.PlayerController|SetbShowMouseCursor _returnvalue_2 false)
    (Input|SetIgnoreLookInput _returnvalue_2 false)
    (Input|SetInputModeGameOnly _returnvalue_2)))

(event Input|ActionEvents|InputActionCrouch
  (params (Key :type Key%20Structure :default "None"))
  ;[1 1 1] Movement Character
  ;;[0 0 0] Crouch
  (:Pressed
    (Utilities|FlowControl|FlipFlop
      (:A
        (Variables|Default|SetCrouch%20Button%20Down true))
      (:B
        (Variables|Default|SetCrouch%20Button%20Down false)))))

(event Input|ActionEvents|InputActionPickUpItem
  (params (Key :type Key%20Structure :default "None"))
  ;[1 1 1] PickUp
  ;;[0 1 0] PickUpItem
  (:Pressed
    (CallFunction|ItemInteractPickUp)))

(event Input|ActionEvents|InputActionMouseClickLeft
  (params (Key :type Key%20Structure :default "None"))
  ;[1 1 1] HUD
  ;;[0.01923 0.02986 1] Selecionar Arma pela HUD
  (:Pressed
    (if (Variables|Default|GetWindowsIsOpen?)
      (bind (_i1 _i2 _i3) (Default|CallSelection (Variables|Default|GetHUDCircularRef)))
      (if _i1
        (if (Utilities|IsValid (Variables|Default|GetAK47))
          (if (and (Variables|Default|GetEquipWeapon) (Variables|Default|GetEquipAK47?))
            (Variables|Default|SetEquipWeapon false)
            (Variables|Default|SetEquipAK47? false)
            (else
              (Variables|Default|SetEquipWeapon true)
              (Variables|Default|SetEquipAK47? true)))
          (Animation|PlayAnimMontage "/Game/Character/Animation/RifleAnimation/EquipAK47.EquipAK47" 1.5 "None"))
        (elif _i3
          (if (Utilities|IsValid (Variables|Default|GetM4A1))
            (if (and (Variables|Default|GetEquipWeapon) (Variables|Default|GetEquipM4A1?))
              (Variables|Default|SetEquipWeapon false)
              (Variables|Default|SetEquipM4A1? false)
              (else
                (Variables|Default|SetEquipWeapon true)
                (Variables|Default|SetEquipM4A1? true)))
            (Animation|PlayAnimMontage "/Game/Character/Animation/RifleAnimation/EquipM4A1.EquipM4A1" 1.5 "None")))))))

(event Input|ActionEvents|InputActionFireWeapon
  (params (Key :type Key%20Structure :default "None"))
  ;[1 1 1] Armas
  ;;[1 0 0] Atirar M4/AK47
  (:Pressed
    (if (and (Variables|Default|GetAinRifle?) (Variables|Default|GetEquipAK47?))
      (if (Utilities|IsValid (Variables|Default|GetAK47))
        (Default|FirePress (Variables|Default|GetAK47)))
      (elif (and (Variables|Default|GetAinRifle?) (Variables|Default|GetEquipM4A1?))
        (if (Utilities|IsValid (Variables|Default|GetM4A1))
          (Default|FirePress (Variables|Default|GetM4A1))))))
  (:Released
    (if (and (Variables|Default|GetAinRifle?) (Variables|Default|GetEquipAK47?))
      (Default|FireReleased (Variables|Default|GetAK47))
      (elif (and (Variables|Default|GetAinRifle?) (Variables|Default|GetEquipM4A1?))
        (Default|FireReleased (Variables|Default|GetM4A1))))))

(event Input|ActionEvents|InputActionReload
  (params (Key :type Key%20Structure :default "None"))
  ;[1 1 1] Armas
  ;;[1 0 0] Reload M4/AK47
  (:Pressed
    (if (or (Variables|Default|GetEquipAK47?) (Variables|Default|GetAinRifle?))
      (if (Utilities|IsValid (Variables|Default|GetAK47))
        (Default|Reload (Variables|Default|GetAK47))
        (else
          (if (Utilities|IsValid (Variables|Default|GetM4A1)) :!label _label
            (Default|Reload (Variables|Default|GetM4A1)))))
      (elif (or (Variables|Default|GetEquipM4A1?) (Variables|Default|GetAinRifle?))
        (goto _label)))))

(event Input|AxisEvents|InputAxisMoveForward
  (params (AxisValue :type Float%20%28single-precision%29))
  ;[1 1 1] Movement Character
  ;;[0 0 0] Movimento W/A/S/D
  (Utilities|SpeedCheck)
  (Pawn|Input|AddMovementInput (Math|Vector|GetForwardVector (Math|Rotator|MakeRotator 0.0 0.0 (.Yaw (Math|Rotator|BreakRotator (Pawn|GetControlRotation :!class /Script/Engine.Pawn))))) AxisValue false))

(event Input|AxisEvents|InputAxisMoveRight
  (params (AxisValue :type Float%20%28single-precision%29))
  ;[1 1 1] Movement Character
  ;;[0 0 0] Movimento W/A/S/D
  (Utilities|SpeedCheck)
  (Pawn|Input|AddMovementInput (Math|Vector|GetRightVector (Math|Rotator|MakeRotator 0.0 0.0 (.Yaw (Math|Rotator|BreakRotator (Pawn|GetControlRotation :!class /Script/Engine.Pawn))))) AxisValue false))

(event Input|AxisEvents|InputAxisMouseX
  (params (AxisValue :type Float%20%28single-precision%29))
  ;[1 1 1] Movement Character
  ;;[0 0 0] Movimento do Mouse
  (Pawn|Input|AddControllerYawInput AxisValue))

(event Input|AxisEvents|InputAxisMouseY
  (params (AxisValue :type Float%20%28single-precision%29))
  ;[1 1 1] Movement Character
  ;;[0 0 0] Movimento do Mouse
  (Pawn|Input|AddControllerPitchInput AxisValue))

(fn ConstructionScript)

(fn ItemDecoration
  (bind (_startlinetrace _endlinetrace) (Utilities|LineTraceValue 2e+02))
  ;[0.08643 1 0] Item
  (bind (_outhit _returnvalue) (Collision|LineTraceByChannel _startlinetrace _endlinetrace "TraceTypeQuery1" false 0 "None"))
  (if _returnvalue
    (bind _asbp_item_base (Utilities|Casting|CastToBP_ItemBase (.HitActor (Collision|BreakHitResult _outhit)))
      (:then
        (if (== _asbp_item_base (.HitActor (Collision|BreakHitResult _outhit)))
          (Variables|Default|SetItemBaseREF _asbp_item_base)
          (Default|WidgetVisibility _asbp_item_base true)
          (CallFunction|CrossHair "Hidden" "Visible")))
      (:CastFailed
        (Utilities|IsValid (Variables|Default|GetItemBaseREF) :!label _label
          (:Is%20Valid
            (bind _output_get (Variables|Default|SetItemBaseREF (Variables|Default|GetItemBaseREF)))
            (Default|WidgetVisibility _output_get false)
            (CallFunction|CrossHair "Visible" "Collapsed")))))
    (else
      (goto _label))))

(fn ItemInteractPickUp
  (bind (_startlinetrace _endlinetrace) (Utilities|LineTraceValue 2e+02))
  (bind (_outhit _returnvalue) (Collision|LineTraceByChannel _startlinetrace _endlinetrace "TraceTypeQuery1" false 0 "None"))
  (if _returnvalue
    (if (Utilities|DoesObjectImplementInterface (.HitActor (Collision|BreakHitResult _outhit)) "/Game/Itens/OutrosBP/ItemInteract.ItemInteract_C")
      (Class|ItemInteract|ItemPickUp(Message) (.HitActor (Collision|BreakHitResult _outhit))))))

(fn CrossHair
  (params (CrossHairNormal :type ESlateVisibility%20Enum :default "Visible") (CrossHairInspec :type ESlateVisibility%20Enum :default "Visible"))
  (Widget|SetVisibility (Variables|/Game/Character/HUD/MainHUD.MainHUD_C|GetCrossHairInspec (Variables|Default|GetMainHudRef)) CrossHairNormal)
  (Widget|SetVisibility (Variables|/Game/Character/HUD/MainHUD.MainHUD_C|GetCrossHairInspec (Variables|Default|GetMainHudRef)) CrossHairInspec))