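; Base item actor for a health pickup that shows a name widget and restores player health when picked up.
; BeginPlay passes the item name to its widget and caches the TPS_Character player reference.
; ItemPickUp adds HealthValue only when health is below 100, without clamping, then destroys the actor and restores the normal crosshair.
; WidgetVisibility toggles the name widget together with the mesh's custom depth rendering for highlighting.
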(event EventBeginPlay
  ;[0.04933 1 0] Name Item
  (bind _asitem_name (Utilities|Casting|CastToItemName (UserInterface|GetUserWidgetObject (Variables|Default|GetItemNameWidget))))
  (Variables|/Game/Itens/HUD/ItemName.ItemName_C|SetItemNameW _asitem_name (Variables|Default|GetItemName))
  (bind _astps_character (Utilities|Casting|CastToTPS_Character (Game|GetPlayerCharacter 0)))
  (Variables|Default|SetTPSCharRef _astps_character))

(event EventItemPickUp
  (bind _tpscharref (Variables|Default|GetTPSCharRef))
  (if (< (Variables|/Game/Character/BluePrints/TPS_Character.TPS_Character_C|GetHealth _tpscharref) 1e+02)
    (bind _output_get (Variables|/Game/Character/BluePrints/TPS_Character.TPS_Character_C|SetHealth _tpscharref (+ (Variables|Default|GetHealth%20Value) (Variables|/Game/Character/BluePrints/TPS_Character.TPS_Character_C|GetHealth _tpscharref))))
    (Development|PrintString (Utilities|String|ToString(Float) _output_get))
    (Actor|DestroyActor self)
    (Default|CrossHair (Variables|Default|GetTPSCharRef) "Visible" "Hidden")))

(fn ConstructionScript)

(fn WidgetVisibility
  (params (Widget%20Eneblad? :type Boolean))
  (Rendering|SetVisibility (Variables|Default|GetItemNameWidget) Widget%20Eneblad? false)
  (Rendering|SetRenderCustomDepth (Variables|Default|GetItemMesh) Widget%20Eneblad?))